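; BP_Turret is a turret actor that turns to face the player character while that character is inside its range.
; Each Tick it checks whether RangeBox overlaps the first player's character.
; If so, it computes a look-at rotation from TurretMesh to the character and keeps only the yaw.
; That world-space yaw is set as the mesh's relative rotation, with pitch and roll zeroed.
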(event `self.ReceiveTick`
  (params (DeltaSeconds :type "Float (single-precision)"))
  (bind _returnvalue (`GameplayStatics.GetPlayerCharacter` 0))
  ;[1 1 1] If character is within box, Look at character
  (if (`PrimitiveComponent.IsOverlappingActor` (`self.RangeBox`) _returnvalue)
    (`SceneComponent.K2_SetRelativeRotation` (`self.TurretMesh`) (`KismetMathLibrary.MakeRotator` 0.0 0.0 (.yaw (`KismetMathLibrary.FindLookAtRotation` (`SceneComponent.K2_GetComponentLocation` (`self.TurretMesh`)) (`self.K2_GetActorLocation` _returnvalue)))) false false)))

(fn `UserConstructionScript`)