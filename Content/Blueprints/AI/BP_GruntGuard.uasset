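; Grunt guard AI character that attacks with a spear and dies as soon as it receives an attack.
; Attack requests play a montage, and the toggleable spear collision sends a zero-value damage message on overlap, then switches off.
; Death detaches the controller, ragdolls mesh and spear, and destroys the actor after a delay.
; Walk speed is randomized at spawn, and unconnected explosion and camera shake effects never run.
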(event `self.ReceiveBeginPlay`
  (bind _charactermovement (`self.CharacterMovement`))
  (set `CharacterMovementComponent.MaxWalkSpeed` (+ (`CharacterMovementComponent.MaxWalkSpeed` _charactermovement) (`KismetMathLibrary.RandomFloatInRange` (* (`self.RandomWalkSpeedDeviation`) -1.0) (`self.RandomWalkSpeedDeviation`))) _charactermovement)
  (`SkinnedMeshComponent.SetPhysicsAsset` (`self.Mesh`) "/Game/Meshes/Mannequin/SK_Mannequin_PhysicsAsset.SK_Mannequin_PhysicsAsset" false))

(event `StartAttackSeqence`
  (`self.PlayAnimMontage` "/Game/Meshes/Mannequin/AnimationsGrunt/GruntGuardAttack_Montage.GruntGuardAttack_Montage" :!label _label)
  (set `self.bIsAttacking` true))

(event `/Game/Blueprints/BP_CombatInterface.StartAttackAI`
  (params (AttackIndex :type Integer))
  (switch `int` AttackIndex
    (:`0`
      (goto _label))))

(event `EnableWeaponCollision`
  (`PrimitiveComponent.SetCollisionEnabled` (`self.Spear`) "QueryAndPhysics"))

(event `self.Spear.OnComponentBeginOverlap`
  (params (OverlappedComponent :type "PrimitiveComponent Object Reference") (OtherActor :type "Actor Object Reference") (OtherComp :type "PrimitiveComponent Object Reference") (OtherBodyIndex :type Integer) (bFromSweep :type Boolean) (SweepResult :type "HitResult Structure (by ref)"))
  ;[1 1 1] Take damage
  (if (not (== OtherActor self))
    (message `/Game/Blueprints/BP_CombatInterface.TakeDamage` OtherActor 0.0 (0.0 0.0 0.0) self)
    (`self.DisableWeaponCollision`)))

(event `DisableWeaponCollision`
  (if (not (`self.bDestroySequenceStarted`))
    (`PrimitiveComponent.SetCollisionEnabled` (`self.Spear`) "NoCollision")))

(event `/Game/Blueprints/BP_CombatInterface.TakeDamage`
  (params (DamageAmountSent :type "Float (single-precision)") (DamageHitDirectionSent :type "Vector Structure") (DamageDealingActor :type "Actor Object Reference")))

(event `ActionAnimStart`
  (set `self.bIsAttacking` true))

(event `ActionAnimEnd`
  (set `self.bIsAttacking` false))

(event `AttackReceived`
  (`self.DestroySequence`))

(event `DestroySequence`
  (set `self.bDestroySequenceStarted` true)
  (`self.StopAnimMontage` "/Game/Meshes/Mannequin/AnimationsGrunt/GruntGuardAttack_Montage.GruntGuardAttack_Montage")
  (`self.DetachFromControllerPendingDestroy`)
  (`PrimitiveComponent.SetCollisionProfileName` (`self.Mesh`) "Ragdoll" false)
  (`PrimitiveComponent.SetCollisionProfileName` (`self.Spear`) "Ragdoll" false)
  (`PrimitiveComponent.SetSimulatePhysics` (`self.Mesh`) true)
  (`PrimitiveComponent.SetSimulatePhysics` (`self.Spear`) true)
  (`PrimitiveComponent.SetCollisionEnabled` (`self.CapsuleComponent`) "NoCollision")
  (`KismetSystemLibrary.Delay` 10.0)
  (`self.K2_DestroyActor`))

(fn `GetIsAttacking`
  (returns (bIsAttacking :type Boolean))
  (return (`self.bIsAttacking`)))

(fn `UserConstructionScript`)