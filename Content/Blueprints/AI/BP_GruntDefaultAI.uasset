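; BP_GruntDefaultAI is the default AI controller for Grunt enemies, linking perception to a behavior tree.
; On BeginPlay it sets up the enemy blackboard, runs the Grunt behavior tree and stores the controlled pawn as SelfActor.
; AI perception updates write any detected BP_PlayerCharacter to PlayerObject, without checking whether the stimulus was gained or lost.
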(event `self.ReceiveBeginPlay`
  (bind _blackboardcomponent (`self.UseBlackboard` "/Game/Blueprints/AI/EnemyBlackboardData.EnemyBlackboardData"))
  (bind _output_get (set `self.CurrentBlackboard` _blackboardcomponent))
  (`self.RunBehaviorTree` "/Game/Blueprints/AI/GruntBehaviorTree.GruntBehaviorTree")
  (`BlackboardComponent.SetValueAsObject` _output_get "SelfActor" (`self.K2_GetPawn`)))

(event `self.AIPerception.OnTargetPerceptionUpdated`
  (params (Actor :type "Actor Object Reference") (Stimulus :type "AIStimulus Structure"))
  (bind _asbp_player_character (cast `/Game/Blueprints/BP_PlayerCharacter` Actor))
  (`BlackboardComponent.SetValueAsObject` (`self.CurrentBlackboard`) "PlayerObject" _asbp_player_character))

(fn `UserConstructionScript`)