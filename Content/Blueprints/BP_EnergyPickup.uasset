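; Energy pickup actor that restores energy points to BP_PlayerCharacter when it overlaps the pickup's Box.
; The Box spins around its yaw axis every Tick at RotationSpeed, scaled by delta time.
; On overlap, it adds PickupEnergy clamped to the player's current max, prints the new total and destroys itself.
; A player already at full energy leaves the pickup in place.
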(event `self.ReceiveTick`
  (params (DeltaSeconds :type "Float (single-precision)"))
  ;[1 1 1] Rotation
  (`SceneComponent.K2_AddLocalRotation` (`self.Box`) (* (`KismetMathLibrary.MakeRotator` 0.0 0.0 (`self.RotationSpeed`)) DeltaSeconds) false false))

(event `self.Box.OnComponentBeginOverlap`
  (params (OverlappedComponent :type "PrimitiveComponent Object Reference") (OtherActor :type "Actor Object Reference") (OtherComp :type "PrimitiveComponent Object Reference") (OtherBodyIndex :type Integer) (bFromSweep :type Boolean) (SweepResult :type "HitResult Structure (by ref)"))
  ;[1 1 1] Add energy on overlap
  (bind _asbp_player_character (cast `/Game/Blueprints/BP_PlayerCharacter` OtherActor))
  (bind _currentenergypoints (`/Game/Blueprints/BP_PlayerCharacter.CurrentEnergyPoints` _asbp_player_character))
  (bind _currentmaxpoints (`/Game/Blueprints/BP_PlayerCharacter.CurrentMaxPoints` _asbp_player_character))
  (if (< _currentenergypoints _currentmaxpoints)
    (bind _returnvalue (+ _currentenergypoints (`self.PickupEnergy`)))
    (if (> _returnvalue _currentmaxpoints)
      (bind _output_get (set `/Game/Blueprints/BP_PlayerCharacter.CurrentEnergyPoints` (`/Game/Blueprints/BP_PlayerCharacter.CurrentMaxPoints` _asbp_player_character) _asbp_player_character))
      (`KismetSystemLibrary.PrintString` (`KismetStringLibrary.Conv_DoubleToString` _output_get))
      (else
        (bind _output_get_2 (set `/Game/Blueprints/BP_PlayerCharacter.CurrentEnergyPoints` _returnvalue _asbp_player_character))
        (`KismetSystemLibrary.PrintString` (`KismetStringLibrary.Conv_DoubleToString` _output_get_2))))
    (`self.K2_DestroyActor`)))

(fn `UserConstructionScript`
  (`parent.UserConstructionScript`))